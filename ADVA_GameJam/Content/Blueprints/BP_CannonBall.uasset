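; Cannonball projectile that explodes on impact and applies damage to the player.
; The construction script sets the projectile movement's X velocity from the Velocity variable.
; Sphere hits on actors tagged Colisionable spawn an explosion emitter and destroy the ball.
; Hits on Player-tagged BP_ThirdPersonCharacter first pass Damage to CambiarVida, then explode the same way; other hits are ignored.
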(event `self.Sphere.OnComponentHit`
  (params (HitComponent :type "PrimitiveComponent Object Reference") (OtherActor :type "Actor Object Reference") (OtherComp :type "PrimitiveComponent Object Reference") (NormalImpulse :type "Vector Structure") (Hit :type "HitResult Structure (by ref)"))
  (if (`self.ActorHasTag` OtherActor "Colisionable")
    (`GameplayStatics.SpawnEmitterAtLocation` "/Game/StarterContent/Particles/P_Explosion.P_Explosion" (`self.K2_GetActorLocation`) :!label _label)
    (`self.K2_DestroyActor`)
    (elif (`self.ActorHasTag` OtherActor "Player")
      (bind _asbp_third_person_character (cast `/Game/ThirdPerson/Blueprints/BP_ThirdPersonCharacter` OtherActor))
      (`/Game/ThirdPerson/Blueprints/BP_ThirdPersonCharacter.CambiarVida` _asbp_third_person_character (`self.Damage`))
      (goto _label))))

(fn `UserConstructionScript`
  (set `MovementComponent.Velocity` (`KismetMathLibrary.MakeVector` (`self.Velocity`)) (`self.ProjectileMovement`)))