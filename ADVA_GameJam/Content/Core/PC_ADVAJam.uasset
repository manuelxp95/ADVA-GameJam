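; Player controller for the ADVA Jam game that manages the player's HUD and the win and death screens.
; On BeginPlay it stores the third-person character, adds the player UI and switches to game-only input.
; Coin and health events forward values to the HUD, caching the coin count.
; Win and death events clear all widgets, show their screen with UI-only input and cursor, and pass it the cached coins.
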(event `self.ReceiveBeginPlay`
  ;[1 1 1] Set UI
  (bind _asbp_third_person_character (cast `/Game/ThirdPerson/Blueprints/BP_ThirdPersonCharacter` (`GameplayStatics.GetPlayerCharacter` 0)))
  (set `self.Player_REF` _asbp_third_person_character)
  (bind _returnvalue (`|CreateWidget` "/Game/UI/WB_PlayerUI.WB_PlayerUI_C"))
  (bind _output_get (set `self.PlayerUI_REF` _returnvalue))
  (`UserWidget.AddToViewport` _output_get 0)
  (`WidgetBlueprintLibrary.SetInputMode_GameOnly` self)
  (set `self.bShowMouseCursor` false))

(event `SetCoins`
  (params (Coins :type Integer))
  (bind _playerui_ref (`self.PlayerUI_REF`))
  (`/Engine/EditorBlueprintResources/StandardMacros.IsValid` _playerui_ref
    (:`Is Valid`
      (`/Game/UI/WB_PlayerUI.Set Coins` _playerui_ref Coins)
      (set `self.MonedasInstancia` Coins))))

(event `SetHealth`
  (params (Health :type "Float (double-precision)"))
  (bind _playerui_ref (`self.PlayerUI_REF`))
  (`/Engine/EditorBlueprintResources/StandardMacros.IsValid` _playerui_ref
    (:`Is Valid`
      (`/Game/UI/WB_PlayerUI.SetHealth in UI` _playerui_ref (`KismetMathLibrary.FTrunc` Health)))))

(event `Death WidgetEnable`
  ;[1 1 1] Lose Screen
  (`WidgetLayoutLibrary.RemoveAllWidgets`)
  (bind _returnvalue (`|CreateWidget` "/Game/UI/WB_DeathUI.WB_DeathUI_C"))
  (`UserWidget.AddToViewport` _returnvalue 0)
  (`WidgetBlueprintLibrary.SetInputMode_UIOnlyEx` self _returnvalue)
  (set `self.bShowMouseCursor` true)
  (`/Game/UI/WB_DeathUI.Set Monedas` _returnvalue (`self.MonedasInstancia`)))

(event `Win WidgetEnabled`
  ;[1 1 1] WinScreen
  (`WidgetLayoutLibrary.RemoveAllWidgets`)
  (bind _returnvalue (`|CreateWidget` "/Game/UI/WB_WinUI.WB_WinUI_C"))
  (`UserWidget.AddToViewport` _returnvalue 0)
  (`WidgetBlueprintLibrary.SetInputMode_UIOnlyEx` self _returnvalue)
  (set `self.bShowMouseCursor` true)
  (`/Game/UI/WB_WinUI.Set Monedas` _returnvalue (`self.MonedasInstancia`)))

(fn `UserConstructionScript`)